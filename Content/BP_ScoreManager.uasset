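; BP_ScoreManager is an actor that tracks the player's score and runs the countdown that ends the game.
; AddScore accumulates points and GetScoreText formats them for display, while StartCountDown starts a looping one-second timer on TickCountdown.
; When time runs out, it sets the game-over flag, clears the timer, shows BP_GameOverWidget with the final score, switches to UI-only input and pauses the game.
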(fn `AddScore`
  (params (Amount :type Integer))
  (set `self.Score` (+ (`self.Score`) Amount)))

(fn `GetScoreText`
  (returns (NewParam :type Text))
  (return (`KismetTextLibrary.Conv_StringToText` (`KismetStringLibrary.Concat_StrStr` "Score: " (`KismetStringLibrary.Conv_IntToString` (`self.Score`))))))

(fn `ShowGameOverUI`
  (bind _returnvalue (`GameplayStatics.GetPlayerController` 0))
  (bind _returnvalue_2 (`|CreateWidget` "/Game/BP_GameOverWidget.BP_GameOverWidget_C"))
  (set `/Game/BP_GameOverWidget.FinalScore` (`self.Score`) _returnvalue_2)
  (`UserWidget.AddToViewport` _returnvalue_2 0)
  (set `PlayerController.bShowMouseCursor` true _returnvalue)
  (`WidgetBlueprintLibrary.SetInputMode_UIOnlyEx` _returnvalue _returnvalue_2)
  (`GameplayStatics.SetGamePaused` true))

(fn `StartCountDown`
  (`KismetSystemLibrary.K2_SetTimer` null "TickCountdown" 1.0 true))

(fn `TickCountdown`
  (bind _countdowntime (`self.CountDownTime`))
  (if (> _countdowntime 0)
    (set `self.CountDownTime` (- _countdowntime 1))
    (else
      (set `self.BGameOver` true)
      (`KismetSystemLibrary.K2_ClearTimer` null "TickCountdown")
      (`self.ShowGameOverUI`))))

(fn `UserConstructionScript`)