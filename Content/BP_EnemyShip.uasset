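; BP_EnemyShip is an enemy ship that circles the player's ship and fires at it once detected.
; DetectionZone overlap stores the player reference and sets an in-range flag, which nothing here clears.
; Tick smoothly turns the ship to a 90-degree yaw offset from the player and orbits by rotating the offset vector, scaled by CurrentRadius.
; A looping BeginPlay timer calls Fire while that flag is set.
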(event `self.ReceiveTick`
  (params (DeltaSeconds :type "Float (single-precision)"))
  (`parent.ReceiveTick` DeltaSeconds)
  (`/Engine/EditorBlueprintResources/StandardMacros.IsValid` (`self.PlayerRef`)
    (:`Is Valid`
      (`|ExecutionSequence`
        (:`then_0`
          (`self.K2_SetActorRotation` (`KismetMathLibrary.RInterpTo` (`self.K2_GetActorRotation`) (`KismetMathLibrary.MakeRotator` (.roll (`KismetMathLibrary.FindLookAtRotation` (`self.K2_GetActorLocation`) (`self.K2_GetActorLocation` (`self.PlayerRef`)))) (.pitch (`KismetMathLibrary.FindLookAtRotation` (`self.K2_GetActorLocation`) (`self.K2_GetActorLocation` (`self.PlayerRef`)))) (+ (.yaw (`KismetMathLibrary.FindLookAtRotation` (`self.K2_GetActorLocation`) (`self.K2_GetActorLocation` (`self.PlayerRef`)))) -90.0)) (`GameplayStatics.GetWorldDeltaSeconds`) 3.0)))
        (:`then_1`
          (`self.K2_SetActorLocation` (+ (`self.K2_GetActorLocation` (`self.PlayerRef`)) (* (`KismetMathLibrary.RotateAngleAxis` (`KismetMathLibrary.Normal` (- (`self.K2_GetActorLocation`) (`self.K2_GetActorLocation` (`self.PlayerRef`)))) (* 30.0 (`GameplayStatics.GetWorldDeltaSeconds`)) (0.0 0.0 1.0)) (`self.CurrentRadius`)))))
        (:`then_2`
          (set `self.CurrentRadius` (`KismetMathLibrary.FInterpTo` (`self.CurrentRadius`) (`KismetMathLibrary.VSize` (- (`self.K2_GetActorLocation`) (`self.K2_GetActorLocation` (`self.PlayerRef`)))) (`GameplayStatics.GetWorldDeltaSeconds`) 1000.0)))))))

(event `self.DetectionZone.OnComponentBeginOverlap`
  (params (OverlappedComponent :type "PrimitiveComponent Object Reference") (OtherActor :type "Actor Object Reference") (OtherComp :type "PrimitiveComponent Object Reference") (OtherBodyIndex :type Integer) (bFromSweep :type Boolean) (SweepResult :type "HitResult Structure (by ref)"))
  (bind _asbp_player_ship (cast `/Game/BP_PlayerShip` OtherActor))
  (`|ExecutionSequence`
    (:`then_0`
      (set `self.PlayerRef` _asbp_player_ship))
    (:`then_1`
      (set `self.IsPlayerInRange` true))))

(event `FireAtPlayer`
  (if (`self.IsPlayerInRange`)
    (`self.Fire`)))

(event `self.ReceiveBeginPlay`
  (`KismetSystemLibrary.K2_SetTimer` null "FireAtPlayer" 3.0 true))

(fn `UserConstructionScript`
  (`parent.UserConstructionScript`))